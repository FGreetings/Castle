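; BP_BulletBase_Net is a bullet actor Blueprint whose own logic stretches its mesh while it exists.
; Each Tick sets the BulletMesh world scale with thin fixed X and Z and Y taken from XScale, then increases XScale by a fixed step, so growth depends on frame rate.
; BeginPlay and overlap events are disabled stubs, and the construction script only calls the parent.
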(event EventBeginPlay
  (|CallParentFunction) ; 此节点被禁用，将不会被调用。\n从引脚连出引线来编译功能。
)

(event Collision|EventActorBeginOverlap
  (params (OtherActor :type Actor%20Object%20Reference)))

(event EventTick
  (params (DeltaSeconds :type Float%20%28single-precision%29))
  (Transformation|SetWorldScale3D (Variables|Default|GetBulletMesh) (Math|Vector|MakeVector 0.1 (Variables|Default|GetX%20Scale) 0.1))
  (Variables|Default|SetX%20Scale (+ (Variables|Default|GetX%20Scale) 0.05)))

(fn ConstructionScript
  (|CallParentFunction))