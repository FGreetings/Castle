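; BP_BulletBase is a projectile that damages enemies on overlap, behaving as a Hit or Net type set by BulletParameter.
; BeginPlay adds projectile movement, then any nonzero lifetime expires into a red material and delayed removal.
; Gated sphere overlaps apply damage: Hit bullets destroy themselves once penetration is spent, while Net bullets attach enemies and pause their move-to-player timers.
; An expiring Net detaches captives, resumes their timers and destroys itself.
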(event OnComponentBeginOverlap(Sphere)
  (params (OverlappedComponent :type Primitive%20Component%20Object%20Reference) (OtherActor :type Actor%20Object%20Reference) (OtherComp :type Primitive%20Component%20Object%20Reference) (OtherBodyIndex :type Integer) (bFromSweep :type Boolean) (SweepResult :type Hit%20Result%20Structure%20%28by%20ref%29))
  (bind _bullet_parameter (Variables|Default|GetBullet%20Parameter))
  (bind (_bullettype _damage _damagedecay _damagetype _penetratenumber) (Utilities|Struct|BreakStruct_Bullet _bullet_parameter))
  (Utilities|FlowControl|Gate false
    (:Exit
      (bind _asbp_enemy_base (Utilities|Casting|CastToBP_EnemyBase OtherActor))
      (switch Utilities|FlowControl|Switch|SwitchonUEnum_BulletType _bullettype
        (:NewEnumerator0
          (Game|Damage|ApplyDamage _asbp_enemy_base _damage 0 0)
          (if (<= _penetratenumber 0)
            (Math|Integer|DecrementInt _penetratenumber
              (:%20%20
                (Actor|DestroyActor)))))
        (:NewEnumerator4
          (Utilities|Array|AddUnique (Variables|Default|GetAttacked%20Enemies) 0)
          (Game|Damage|ApplyDamage _asbp_enemy_base 0.0 0 0)
          (CallFunction|NetAttack _asbp_enemy_base))))))

(event Custom|Release%20all%20enemy
  (for _array_element (Variables|Default|GetAttacked%20Enemies)
    (Transformation|DetachFromActor _array_element "KeepWorld" "KeepWorld" "KeepWorld")
    (Class|KismetSystemLibrary|UnPauseTimer _array_element "MoveToPlayerFunc"))
  (Actor|DestroyActor))

(event Custom|MoveFunc
  (bind _bullet_parameter (Variables|Default|GetBullet%20Parameter))
  (bind (_bullettype _damage _damagedecay _damagetype _penetratenumber _chainnumber _initialspeed _maxspeed) (Utilities|Struct|BreakStruct_Bullet _bullet_parameter))
  (bind _returnvalue (AddComponent|AddProjectileMovementComponent))
  (Variables|/Script/Engine.ProjectileMovementComponent|SetInitialSpeed _returnvalue _initialspeed)
  (Variables|/Script/Engine.ProjectileMovementComponent|SetMaxSpeed _returnvalue _maxspeed))

(event Custom|Net%20Attack
  (params (Target%20Enemy :type BP%20Enemy%20Base%20Object%20Reference))
  (Class|KismetSystemLibrary|PauseTimer Target%20Enemy "MoveToPlayerFunc")
  (Transformation|AttachActorToActor Target%20Enemy self "None" "KeepWorld" "KeepWorld" "KeepWorld" false))

(event EventBeginPlay
  (bind _bullet_parameter (Variables|Default|GetBullet%20Parameter))
  (bind _bullet_parameter_2 (Variables|Default|GetBullet%20Parameter))
  (bind (_bullettype _damage _damagedecay _damagetype _penetratenumber) (Utilities|Struct|BreakStruct_Bullet _bullet_parameter))
  (bind (_bullettype_2 _damage_2 _damagedecay_2 _damagetype_2 _penetratenumber_2 _chainnumber _initialspeed _maxspeed _bulletduration _deadduration) (Utilities|Struct|BreakStruct_Bullet _bullet_parameter_2))
  (CallFunction|MoveFunc)
  (if (!= _bulletduration 0.0)
    (Utilities|FlowControl|Delay _bulletduration)
    (Rendering|Material|SetMaterial (Variables|Default|GetBulletMesh) 0 "/Game/Mat/M_BaseColor_ECRed.M_BaseColor_ECRed")
    (switch Utilities|FlowControl|Switch|SwitchonUEnum_BulletType (.BulletType (Utilities|Struct|BreakStruct_Bullet (Variables|Default|GetBullet%20Parameter)))
      (:NewEnumerator0
        (Utilities|FlowControl|Delay _deadduration)
        (Actor|DestroyActor))
      (:NewEnumerator4
        (Utilities|FlowControl|Delay _deadduration)
        (CallFunction|ReleaseAllEnemy)
        (Utilities|FlowControl|Gate false) ; enters at Close
      ))))

(fn ConstructionScript)