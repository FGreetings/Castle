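; Castle game mode that runs timed enemy waves alternating with an upgrade stage.
; InitWave recenters the player at BP_OriginPoint and starts looping timers for countdown and spawning.
; Each spawn tick places random base or Crasher enemies in the origin's box, with counts from an arctangent wave curve plus random variance.
; At countdown end, SettleAWave stops timers, clears enemies, banks loot money/exp and shows the upgrade UI.
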(event Custom|CountDown
  (bind _result (Math|Integer|DecrementInt (Variables|Default|GetTimerCount))
    (:%20%20
      (if (<= _result 0)
        (CallFunction|SettleAWave)))))

(event Custom|SpawnEnemies
  (bind _returnvalue (Math|Random|RandomInteger 999))
  (bind _originref (Variables|Default|GetOriginRef))
  (bind _waveindex (Variables|Default|GetWaveIndex))
  (bind _returnvalue_2 (Transformation|GetActorLocation _originref))
  (bind _returnvalue_3 (Math|Random|MakeRandomStream _returnvalue))
  (bind _returnvalue_4 (* _waveindex 5))
  (bind _in_box_extent (Variables|/Game/BP/BP_OriginPoint.BP_OriginPoint_C|GetIn%20Box%20Extent _originref))
  (bind _returnvalue_5 (Class|KismetMathLibrary|RandomPointinBoundingBoxfromStream _returnvalue_2 _in_box_extent _returnvalue_3))
  ;[1 1 1] 随机范围内生成AI
  (for _index (range 0 (Math|Integer|Clamp(Integer) (+ (|(Ceil((3*((arctan((a-10)))+2)))) (Math|Conversions|ToFloat(Integer) (Variables|Default|GetWaveIndex))) (Math|Random|RandomIntegerinRange (* _returnvalue_4 -1) _returnvalue_4)) 1 9999))
    (switch int (Math|Random|RandomIntegerinRange 0 1)
      (:Default
        (Game|SpawnActorfromClass "/Game/BP/Enemy/BP_EnemyBase.BP_EnemyBase_C" (Math|Transform|MakeTransform _returnvalue_5 "0, 0, 0" "1.000000,1.000000,1.000000") "Undefined" 0 0 :!label _label))
      (:0
        (goto _label))
      (:1
        (Game|SpawnActorfromClass "/Game/BP/Enemy/BP_EnemyBase_TheCrasher.BP_EnemyBase_TheCrasher_C" (Math|Transform|MakeTransform _returnvalue_5 "0, 0, 0" "1.000000,1.000000,1.000000") "Undefined" 0 0)))))

(event Custom|InitWave
  (bind _returnvalue (Game|GetPlayerController 0))
  (Utilities|FlowControl|Sequence
    (:then_0
      (Variables|Default|SetTimerCount (Variables|Default|GetDefaultTimer))
      (Math|Integer|IncrementInt (Variables|Default|GetWaveIndex)))
    (:then_1
      (bind _returnvalue_2 (Actor|GetActorOfClass "/Game/BP/BP_OriginPoint.BP_OriginPoint_C"))
      (Transformation|SetActorLocation (Game|Player|GetPlayerPawn 0) (Transformation|GetActorLocation _returnvalue_2) false false))
    (:then_2
      (CallFunction|CountDown)
      (Utilities|Time|SetTimerbyFunctionName 0 "CountDown" 1.0 true 1.0))
    (:then_3
      (Utilities|Time|SetTimerbyFunctionName 0 "SpawnEnemies" 1.0 true))
    (:then_4
      (Widget|SetVisibility (Variables|Default|GetMainUI) "Visible")
      (Widget|SetVisibility (Variables|Default|GetUpgradeUIRef) "Collapsed"))
    (:then_5
      (bind _asbp_castle_base (Utilities|Casting|CastToBP_CastleBase (Game|Player|GetPlayerPawn 0)))
      (Default|Into/OutUpgradeStage _asbp_castle_base false))
    (:then_6
      (Input|SetInputModeGameandUI _returnvalue 0 "DoNotLock" true)
      (Variables|/Script/Engine.PlayerController|SetbShowMouseCursor _returnvalue false))))

(event Custom|SettleAWave
  (Utilities|FlowControl|Sequence
    (:then_0
      ;[1 1 1] 清除计时器
      (Utilities|Time|ClearTimerbyFunctionName 0 "CountDown")
      (Utilities|Time|ClearTimerbyFunctionName 0 "SpawnEnemies"))
    (:then_1
      (bind _outactors (Actor|GetAllActorsOfClass "/Game/BP/Enemy/BP_EnemyBase.BP_EnemyBase_C"))
      (for _array_element _outactors
        (Actor|DestroyActor)))
    (:then_2
      (bind _outactors_2 (Actor|GetAllActorsOfClass "/Game/BP/Enemy/BP_Loot.BP_Loot_C"))
      (for _array_element_2 _outactors_2
        (Default|AddMoney&ExptoPlayer _array_element_2)))
    (:then_3
      (Widget|SetVisibility (Variables|Default|GetUpgradeUIRef) "Visible"))
    (:then_4
      (bind _asbp_castle_base (Utilities|Casting|CastToBP_CastleBase (Game|Player|GetPlayerPawn 0)))
      (Default|Into/OutUpgradeStage _asbp_castle_base true))
    (:then_5
      (Variables|/Script/Engine.PlayerController|SetbShowMouseCursor (Game|GetPlayerController 0) true))
    (:then_6
      (bind _outactors_3 (Actor|GetAllActorsOfClass "/Game/BP/Enemy/BP_EnemyBase.BP_EnemyBase_C"))
      (for _array_element_3 _outactors_3
        (Actor|DestroyActor _array_element_3)))))

(event EventBeginPlay
  ;[1 1 1] Init
  (Utilities|FlowControl|Sequence
    (:then_0
      (bind _returnvalue (UserInterface|CreateWidget "/Game/BP/UI/WBP_MainUI.WBP_MainUI_C"))
      (bind _output_get (Variables|Default|SetMainUI _returnvalue))
      (UserInterface|Viewport|AddtoViewport _output_get 0)
      (Widget|SetVisibility _output_get "Collapsed"))
    (:then_1
      (bind _returnvalue_2 (UserInterface|CreateWidget "/Game/BP/UI/WBP_Upgrade.WBP_Upgrade_C"))
      (bind _output_get_2 (Variables|Default|SetUpgradeUIRef _returnvalue_2))
      (UserInterface|Viewport|AddtoViewport _returnvalue_2 0)
      (Widget|SetVisibility _output_get_2 "Collapsed"))
    (:then_2
      (bind _returnvalue_3 (Actor|GetActorOfClass "/Game/BP/BP_OriginPoint.BP_OriginPoint_C"))
      (Variables|Default|SetOriginRef _returnvalue_3))))

(fn ConstructionScript)