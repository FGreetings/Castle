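; Castle player controller that handles grid-snapped building placement on the player's castle pawn.
; SpawnBuilding creates a preview, replacing any pending one, which Tick snaps slightly above the grid cell nearest a mouse trace from the upgrade camera.
; The preview's marker shows whether that cell, found through the castle's grid manager component, is free.
; Left click on a free cell places the building, marks it occupied and attaches it to the pawn.
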(event Custom|SpawnBuilding
  (params (BuildingsClass :type BP%20Construction%20Base%20Class%20Reference))
  (bind _spawnedconstructionref (Variables|Default|GetSpawnedConstructionRef)
    (:then
      (Actor|DestroyActor _spawnedconstructionref))
    (:else
      _))
  (bind _returnvalue (Game|SpawnActorfromClass BuildingsClass (Math|Transform|MakeTransform "0, 0, 0" "0, 0, 0" "1.000000,1.000000,1.000000") "Undefined" 0 0))
  (Variables|Default|SetConstructionSpawned? true)
  (Variables|Default|SetSpawnedConstructionRef _returnvalue))

(event EventTick
  (params (DeltaSeconds :type Float%20%28single-precision%29))
  (if (Variables|Default|GetConstructionSpawned?)
    (CallFunction|SetBuildingPlacement)
    (CallFunction|SetBuildingBuildState)))

(event Input|MouseEvents|LeftMouseButton
  (params (Key :type Key%20Structure :default "None"))
  (:Pressed
    (bind _spawnedconstructionref (Variables|Default|GetSpawnedConstructionRef)
      (:then
        (bind (_closestgrid _closestlocation) (CallFunction|GetClosestGridInfo))
        (if (not (Variables|/Game/BP/Castle/BP_BuildingGridBase.BP_BuildingGridBase_C|GetHadAnyBuilding? _closestgrid))
          (Transformation|SetActorLocation _spawnedconstructionref _closestlocation false false)
          (Variables|/Game/BP/Castle/BP_BuildingGridBase.BP_BuildingGridBase_C|SetHadAnyBuilding? _closestgrid true)
          (Transformation|AttachActorToActor _spawnedconstructionref (Game|Player|GetPlayerPawn 0) "None" "KeepWorld" "KeepRelative" "KeepRelative" true)
          (Default|UpdateBuildingStateMarker _spawnedconstructionref false false)
          (Variables|Default|SetSpawnedConstructionRef 0)))
      (:else))))

(fn ConstructionScript)

(fn SetBuildingPlacement
  (bind _closestlocation (CallFunction|GetClosestGridInfo))
  (bind _spawnedconstructionref (Variables|Default|GetSpawnedConstructionRef)
    (:then
      (Transformation|SetActorLocation _spawnedconstructionref (Math|Vector|MakeVector (.X (Math|Vector|BreakVector _closestlocation)) (.Y (Math|Vector|BreakVector _closestlocation)) (+ (.Z (Math|Vector|BreakVector _closestlocation)) 15.0)) false false))
    (:else)))

(fn GetMouseLocationinWorld
  (bind (_worldlocation _worlddirection) (Game|Player|ConvertMouseLocationToWorldSpace))
  (bind _asbp_castle_base (Utilities|Casting|CastToBP_CastleBase (Game|Player|GetPlayerPawn 0))
    (:then
      (bind _outhit (Collision|LineTraceByChannel (Transformation|GetWorldLocation (Variables|/Game/BP/Castle/BP_CastleBase.BP_CastleBase_C|GetUpgradeCamera _asbp_castle_base)) (+ _worldlocation (* _worlddirection 1e+04)) "TraceTypeQuery1" false 0 "None")))
    (:CastFailed
      _))
  (return (.Location (Collision|BreakHitResult _outhit))))

(fn SetBuildingBuildState
  (bind _closestgrid (CallFunction|GetClosestGridInfo))
  (bind _spawnedconstructionref (Variables|Default|GetSpawnedConstructionRef)
    (:then
      (Default|UpdateBuildingStateMarker _spawnedconstructionref true (not (Variables|/Game/BP/Castle/BP_BuildingGridBase.BP_BuildingGridBase_C|GetHadAnyBuilding? _closestgrid))))
    (:else)))

(fn GetClosestGridInfo
  (bind _asbp_castle_base (Utilities|Casting|CastToBP_CastleBase (Game|Player|GetPlayerPawn 0))
    (:then
      (bind _location (CallFunction|GetMouseLocationinWorld))
      (bind (_closestgrid _closestlocation _closestdistance) (Default|GetClosestGridLocation (Variables|/Game/BP/Castle/BP_CastleBase.BP_CastleBase_C|GetBP_BuildingGridManagerComp _asbp_castle_base) _location)))
    (:CastFailed
      _))
  (return _closestgrid _closestlocation _closestdistance))