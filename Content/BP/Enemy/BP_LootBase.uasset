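; BP_LootBase is a loot pickup that flies to the player's castle and grants loot, coin and experience.
; When its Sphere overlaps a BP_CastleBase, it either collects immediately if touching the castle's Base, or starts a looping timer.
; The timer turns it toward the player pawn on yaw and steps it forward.
; Collection passes LootSetting values to the castle's Loot function, then destroys the actor.
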(event OnComponentBeginOverlap(Sphere)
  (params (OverlappedComponent :type Primitive%20Component%20Object%20Reference) (OtherActor :type Actor%20Object%20Reference) (OtherComp :type Primitive%20Component%20Object%20Reference) (OtherBodyIndex :type Integer) (bFromSweep :type Boolean) (SweepResult :type Hit%20Result%20Structure%20%28by%20ref%29))
  (bind _asbp_castle_base (Utilities|Casting|CastToBP_CastleBase OtherActor))
  (if (Collision|IsOverlappingActor (Variables|/Game/BP/Castle/BP_CastleBase.BP_CastleBase_C|GetBase _asbp_castle_base) self :!class /Script/Engine.PrimitiveComponent)
    (CallFunction|AddMoney&ExptoPlayer)
    (else
      (Utilities|Time|SetTimerbyFunctionName 0 "MoveToCastle" 0.01 true))))

(event Custom|AddMoney&ExpToPlayer
  (bind _lootsetting (Variables|Default|GetLootSetting))
  (bind _asbp_castle_base (Utilities|Casting|CastToBP_CastleBase (Game|Player|GetPlayerPawn 0)))
  (Default|Loot _asbp_castle_base 1 (Utilities|Array|Get(acopy) _lootsetting) (Utilities|Array|Get(acopy) _lootsetting 1) (Utilities|Array|Get(acopy) _lootsetting 2))
  (Actor|DestroyActor))

(event Custom|MoveToCastle
  (Transformation|SetActorRotation (Math|Interpolation|RInterpTo (Transformation|GetActorRotation) (Math|Rotator|MakeRotator 0.0 0.0 (.Yaw (Math|Rotator|BreakRotator (Math|Rotator|FindLookatRotation (Transformation|GetActorLocation) (Transformation|GetActorLocation (Game|Player|GetPlayerPawn 0)))))) (Utilities|Time|GetWorldDeltaSeconds) 5e+01))
  (Transformation|AddActorLocalOffset (Math|Vector|MakeVector 5e+01 0.0 0.0) false false))

(fn ConstructionScript)