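; Enemy base actor that homes in on the player pawn and deals random damage to the castle.
; A fast looping timer, started after a short delay, yaws it toward the player and steps it forward without sweep.
; Incoming damage updates a widget health bar; death scatters random BP_Loot nearby and destroys it.
; Its sphere overlapping BP_CastleBase's DamageArea applies damage and destroys the enemy without dropping loot.
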(event OnComponentBeginOverlap(Sphere)
  (params (OverlappedComponent :type Primitive%20Component%20Object%20Reference) (OtherActor :type Actor%20Object%20Reference) (OtherComp :type Primitive%20Component%20Object%20Reference) (OtherBodyIndex :type Integer) (bFromSweep :type Boolean) (SweepResult :type Hit%20Result%20Structure%20%28by%20ref%29))
  ;[1 1 1] 施加伤害
  (bind _asbp_castle_base (Utilities|Casting|CastToBP_CastleBase OtherActor))
  (if (== (Variables|/Game/BP/Castle/BP_CastleBase.BP_CastleBase_C|GetDamageArea _asbp_castle_base) OtherComp)
    (Game|Damage|ApplyDamage _asbp_castle_base (Math|Conversions|ToFloat(Integer) (Math|Random|RandomIntegerinRange 1 5)) 0 0)
    (Actor|DestroyActor)))

(event Custom|MoveToPlayerFunc
  ;[1 1 1] 向玩家移动
  (Transformation|SetActorRotation (Math|Interpolation|RInterpTo (Transformation|GetActorRotation) (Math|Rotator|MakeRotator 0.0 0.0 (.Yaw (Math|Rotator|BreakRotator (Math|Rotator|FindLookatRotation (Transformation|GetActorLocation) (Transformation|GetActorLocation (Game|Player|GetPlayerPawn 0)))))) (Utilities|Time|GetWorldDeltaSeconds) 5e+01))
  (Transformation|AddActorLocalOffset (Math|Vector|MakeVector (Variables|Default|GetMovement) 0.0 0.0) false false))

(event Custom|DeathEvent
  ;[1 1 1] 死亡事件
  (for _index (range 0 (Math|Random|RandomIntegerinRange 1 4))
    (Game|SpawnActorfromClass "/Game/BP/Enemy/BP_Loot.BP_Loot_C" (Math|Transform|MakeTransform (Math|Random|RandomPointinBoundingBox (Transformation|GetActorLocation) "100.000000,100.000000,0.000000")) "Undefined" 0 0)
    (Actor|DestroyActor)))

(event Game|Damage|EventAnyDamage
  (params (Damage :type Float%20%28single-precision%29) (DamageType :type Damage%20Type%20Object%20Reference) (InstigatedBy :type Controller%20Object%20Reference) (DamageCauser :type Actor%20Object%20Reference))
  (bind _widget (Variables|Default|GetWidget))
  ;[1 1 1] 伤害检测
  (bind _output_get (Variables|Default|SetHP (- (Variables|Default|GetHP) Damage)))
  (Utilities|FlowControl|Sequence
    (:then_0
      (if (<= _output_get 0.0)
        (CallFunction|DeathEvent)))
    (:then_1
      (Utilities|IsValid _widget
        (:Is%20Valid
          (bind _aswbp_enemy_hpbar (Utilities|Casting|CastToWBP_EnemyHPBar (UserInterface|GetUserWidgetObject _widget)))
          (Progress|SetPercent (Variables|/Game/BP/UI/Enemy/WBP_EnemyHPBar.WBP_EnemyHPBar_C|GetHPBar _aswbp_enemy_hpbar) (/ (Variables|Default|GetHP) (Variables|Default|GetMaxHp))))))))

(event EventBeginPlay
  (Utilities|FlowControl|Delay 0.2)
  (Utilities|Time|SetTimerbyFunctionName self "MoveToPlayerFunc" 0.01 true)
  (bind _aswbp_enemy_hpbar (Utilities|Casting|CastToWBP_EnemyHPBar (UserInterface|GetUserWidgetObject (Variables|Default|GetWidget))))
  (Progress|SetPercent (Variables|/Game/BP/UI/Enemy/WBP_EnemyHPBar.WBP_EnemyHPBar_C|GetHPBar _aswbp_enemy_hpbar) 1.0))

(fn ConstructionScript)