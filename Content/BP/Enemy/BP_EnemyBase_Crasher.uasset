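; Crasher enemy Blueprint that performs a charging attack when its capsule overlaps a BP_CastleBase actor, limited by a cooldown.
; CrashAttack halts movement, briefly enlarges the mesh as a wind-up, pauses the MoveToPlayerFunc timer and computes a yaw toward the player pawn using a single interpolation step.
; A fast looping Crash timer holds that rotation and pushes the actor forward without sweep for a fixed duration, then normal pursuit resumes.
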(event OnComponentBeginOverlap(Capsule_0)
  (params (OverlappedComponent :type Primitive%20Component%20Object%20Reference) (OtherActor :type Actor%20Object%20Reference) (OtherComp :type Primitive%20Component%20Object%20Reference) (OtherBodyIndex :type Integer) (bFromSweep :type Boolean) (SweepResult :type Hit%20Result%20Structure%20%28by%20ref%29))
  (Utilities|Casting|CastToBP_CastleBase OtherActor)
  (if (Variables|Default|GetAble%20to%20Attack)
    (CallFunction|CrashAttack)
    (Variables|Default|SetAble%20to%20Attack false)
    (Utilities|FlowControl|Delay (Variables|Default|GetAttack%20CoolDown))
    (Variables|Default|SetAble%20to%20Attack true)))

(event Custom|Crash
  (Transformation|SetActorRotation (Variables|Default|GetCrash%20Rotation))
  (Transformation|AddActorLocalOffset (Math|Vector|MakeVector 2e+01 0.0 0.0) false false))

(event Custom|Crash%20Attack
  (bind _staticmesh (Variables|Default|GetStaticMesh))
  (Variables|Default|SetMovement 0.0)
  (Transformation|SetRelativeScale3D _staticmesh "1.200000,1.200000,1.200000")
  (Utilities|FlowControl|Delay 0.5)
  (Transformation|SetRelativeScale3D _staticmesh "1.000000,1.000000,1.000000")
  (Class|KismetSystemLibrary|PauseTimer 0 "MoveToPlayerFunc")
  (Variables|Default|SetCrash%20Rotation (Math|Interpolation|RInterpTo (Transformation|GetActorRotation) (Math|Rotator|MakeRotator 0.0 0.0 (.Yaw (Math|Rotator|BreakRotator (Math|Rotator|FindLookatRotation (Transformation|GetActorLocation) (Transformation|GetActorLocation (Game|Player|GetPlayerPawn 0)))))) (Utilities|Time|GetWorldDeltaSeconds) 5e+01))
  (Utilities|Time|SetTimerbyFunctionName 0 "Crash" 0.01 true)
  (Utilities|FlowControl|Delay 2.0)
  (Utilities|Time|ClearTimerbyFunctionName 0 "Crash")
  (Variables|Default|SetMovement 3.0)
  (Class|KismetSystemLibrary|UnPauseTimer 0 "MoveToPlayerFunc"))

(event EventBeginPlay
  (|CallParentFunction) ; 此节点被禁用，将不会被调用。\n从引脚连出引线来编译功能。
)

(event Collision|EventActorBeginOverlap
  (params (OtherActor :type Actor%20Object%20Reference)))

(event EventTick
  (params (DeltaSeconds :type Float%20%28single-precision%29)))

(fn ConstructionScript)