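; Enemy Blueprint that merges same-level pairs into a larger enemy, up to level 2, with Level setting scale, health and speed.
; TrackSphere overlap picks a partner and starts looping timers that steer toward it and watch its validity.
; MergeSphere contact starts a two-second merge phase, then both are destroyed.
; An object-name suffix comparison elects the main merger, which spawns the next-level enemy.
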(event OnComponentBeginOverlap(TrackSphere)
  (params (OverlappedComponent :type Primitive%20Component%20Object%20Reference) (OtherActor :type Actor%20Object%20Reference) (OtherComp :type Primitive%20Component%20Object%20Reference) (OtherBodyIndex :type Integer) (bFromSweep :type Boolean) (SweepResult :type Hit%20Result%20Structure%20%28by%20ref%29))
  (bind _self self)
  (bind _level (Variables|Default|GetLevel))
  (bind _returnvalue (Utilities|GetObjectName _self))
  (bind _returnvalue_2 (Utilities|String|RightChop _returnvalue 22))
  (bind _asbp_enemy_base_merger (Utilities|Casting|CastToBP_EnemyBase_Merger OtherActor))
  (if (not (== OtherActor self))
    (if (Math|Boolean|ANDBoolean (Variables|Default|GetCanMerge) (Variables|BP_EnemyBase_Merger_C|GetCanMerge _asbp_enemy_base_merger) (== _level (Variables|BP_EnemyBase_Merger_C|GetLevel _asbp_enemy_base_merger)) (< _level 2))
      (Variables|Default|SetMergeTarget _asbp_enemy_base_merger)
      (Utilities|Time|SetTimerbyFunctionName 0 "MergeCheck" 0.01 true)
      (Utilities|Time|SetTimerbyFunctionName 0 "TrackOther" 0.01 true)
      (Utilities|FlowControl|Sequence
        (:then_0
          (if (Utilities|Enum|Equal(Enum) _returnvalue_2 "")
            (Variables|BP_EnemyBase_Merger_C|SetMainMerger (Variables|Default|GetMergeTarget) true :!label _label)
            (else
              (if (Utilities|Enum|Equal(Enum) (Utilities|String|RightChop (Utilities|GetObjectName (Variables|Default|GetMergeTarget)) 22) "")
                _
                (elif (> (Math|Conversions|ToInteger(Byte) _returnvalue_2) (Math|Conversions|ToInteger(Byte) (Utilities|String|RightChop (Utilities|GetObjectName (Variables|Default|GetMergeTarget)) 22)))
                  _
                  (else
                    (goto _label))))
              (Variables|Default|SetMainMerger self true))))
        (:then_1
          (Utilities|FlowControl|Delay 0.1)
          (Variables|Default|SetCanMerge false)
          (CallFunction|SetMovementState false))))))

(event OnComponentBeginOverlap(MergeSphere)
  (params (OverlappedComponent :type Primitive%20Component%20Object%20Reference) (OtherActor :type Actor%20Object%20Reference) (OtherComp :type Primitive%20Component%20Object%20Reference) (OtherBodyIndex :type Integer) (bFromSweep :type Boolean) (SweepResult :type Hit%20Result%20Structure%20%28by%20ref%29))
  (bind _mergetarget (Variables|Default|GetMergeTarget))
  (Utilities|IsValid _mergetarget
    (:Is%20Valid
      (if (and (== OtherComp (Variables|BP_EnemyBase_Merger_C|GetMergeSphere _mergetarget)) (< (Variables|Default|GetLevel) 2))
        (Utilities|Time|ClearTimerbyFunctionName 0 "TrackOther")
        (CallFunction|StartMerge)))))

(event Custom|StartMerge
  (Utilities|Time|SetTimerbyFunctionName 0 "MergeAnim" 0.01 true)
  (Utilities|FlowControl|Delay 2.0)
  (Utilities|Time|ClearTimerbyFunctionName 0 "MergeAnim")
  (CallFunction|MergeSuc))

(event Custom|TrackOther
  (Transformation|SetActorRotation (Math|Interpolation|RInterpTo (Transformation|GetActorRotation) (Math|Rotator|MakeRotator 0.0 0.0 (.Yaw (Math|Rotator|BreakRotator (Math|Rotator|FindLookatRotation (Transformation|GetActorLocation) (Transformation|GetActorLocation (Variables|Default|GetMergeTarget)))))) (Utilities|Time|GetWorldDeltaSeconds) 5e+01))
  (Transformation|AddActorLocalOffset (Math|Vector|MakeVector (Variables|Default|GetMovement) 0.0 0.0) false false))

(event Custom|MergeCheck
  (Utilities|IsValid (Variables|Default|GetMergeTarget)
    (:Is%20Not%20Valid
      (Variables|Default|SetMerge%20Failed false)
      (Utilities|FlowControl|Sequence
        (:then_0
          (Utilities|Time|ClearTimerbyFunctionName 0 "MergeCheck"))
        (:then_1
          (Utilities|Time|ClearTimerbyFunctionName 0 "MergeAnim"))
        (:then_2
          (Utilities|Time|ClearTimerbyFunctionName 0 "TrackOther"))))))

(event Custom|MergeSuc
  (Utilities|Time|ClearTimerbyFunctionName 0 "MergeAnim")
  (if (Variables|Default|GetMainMerger)
    (Game|SpawnActorfromClass "BP_EnemyBase_Merger_C" (Math|Transform|MakeTransform (Transformation|GetActorLocation)) "AlwaysSpawn" 0 (+ (Variables|Default|GetLevel) 1) 0)
    (Actor|DestroyActor)
    (else
      (Utilities|FlowControl|Delay 0.1)
      (Actor|DestroyActor))))

(event Custom|MergeAnim
  (Transformation|SetActorRotation "0,10.000000, 0"))

(event Custom|Restart
  (Utilities|FlowControl|Delay 0.5)
  (CallFunction|SetMovementState true))

(event EventBeginPlay
  (|CallParentFunction) ; 此节点被禁用，将不会被调用。\n从引脚连出引线来编译功能。
)

(event Collision|EventActorBeginOverlap
  (params (OtherActor :type Actor%20Object%20Reference)))

(event EventTick
  (params (DeltaSeconds :type Float%20%28single-precision%29)))

(fn ConstructionScript
  (|CallParentFunction)
  (switch int (Variables|Default|GetLevel)
    (:Default
      (Transformation|SetWorldScale3D (Variables|Default|GetStaticMesh) "2.250000,2.250000,2.250000" :!label _label)
      (Variables|Default|SetMaxHp 8.0)
      (Variables|Default|SetHP 8.0)
      (Variables|Default|SetMovement 8.0)
      (Variables|Default|SetCanMerge false))
    (:0
      (Transformation|SetWorldScale3D (Variables|Default|GetStaticMesh) "0.750000,0.750000,0.750000"))
    (:1
      (Transformation|SetWorldScale3D (Variables|Default|GetStaticMesh) "1.500000,1.500000,1.500000")
      (Variables|Default|SetMaxHp 4.0)
      (Variables|Default|SetHP 4.0)
      (Variables|Default|SetMovement 6.0))
    (:2
      (goto _label))))