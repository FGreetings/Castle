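; BP_SpawnerBase_Enemy is an enemy spawner that spawns an actor of its SpawnType class at its own transform.
; Its SpawnEvent casts the player pawn to BP_CastleBase and skips the spawn while the spawner's Capsule overlaps the castle's DamageArea.
; The parent SpawnEvent runs after that check whether or not a spawn happened, but not if the cast fails.
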(event EventBeginPlay
  (|CallParentFunction) ; This node is disabled and will not be called.\nDrag off pins to build functionality.
)

(event Collision|EventActorBeginOverlap
  (params (OtherActor :type Actor%20Object%20Reference))
  (|CallParentFunction OtherActor) ; This node is disabled and will not be called.\nDrag off pins to build functionality.
)

(event EventTick
  (params (DeltaSeconds :type Float%20%28single-precision%29))
  (|CallParentFunction DeltaSeconds) ; This node is disabled and will not be called.\nDrag off pins to build functionality.
)

(fn ConstructionScript
  (|CallParentFunction))

(fn SpawnEvent
  (bind _asbp_castle_base (Utilities|Casting|CastToBP_CastleBase (Game|Player|GetPlayerPawn 0)))
  (if (Class|PrimitiveComponent|IsOverlappingComponent (Variables|/Game/BP/Castle/BP_CastleBase.BP_CastleBase_C|GetDamageArea _asbp_castle_base) (Variables|Default|GetCapsule))
    _
    (else
      (Game|SpawnActorfromClass (Variables|Default|GetSpawnType) (Transformation|GetActorTransform) "Undefined" 0 0)))
  (|CallParentFunction))