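; Base pawn for the player-controlled castle, handling movement, health, loot pickup and an upgrade stage.
; MovementMethod selects Directly Move, Tank or Drone handling, tuning FloatingPawnMovement at construction and routing axis input to matching movement logic.
; The upgrade stage swaps cameras, locks movement and populates the building grid component.
; Damage destroys it below zero HP, loot credits game mode money, and damage, loot and level-up hooks are empty.
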(event Custom|Into/OutUpgradeStage
  (params (In%20Upgrade? :type Boolean))
  (if In%20Upgrade?
    (Components|Activation|Deactivate (Variables|Default|GetGameCamera))
    (Components|Activation|Activate (Variables|Default|GetUpgradeCamera) false)
    (Variables|Status|SetCanMove false)
    (Default|PopulateGrid (Variables|Default|GetBP_BuildingGridManagerComp))
    (else
      (Components|Activation|Deactivate (Variables|Default|GetUpgradeCamera))
      (Components|Activation|Activate (Variables|Default|GetGameCamera) false)
      (Variables|Status|SetCanMove true))))

(event Game|Damage|EventAnyDamage
  (params (Damage :type Float%20%28single-precision%29) (DamageType :type Damage%20Type%20Object%20Reference) (InstigatedBy :type Controller%20Object%20Reference) (DamageCauser :type Actor%20Object%20Reference))
  ;[1 1 1] 伤害鉴定
  (bind _output_get (Variables|OAttribute|SetHP (- (Variables|OAttribute|GetHP) Damage)))
  (CallFunction|DamagedEvent DamageType DamageCauser)
  (if (< _output_get 0.0)
    (Actor|DestroyActor)))

(event EventTick
  (params (DeltaSeconds :type Float%20%28single-precision%29))
  (Development|PrintString (Utilities|String|Append "Player HP：" (Utilities|String|ToString(Float) (Variables|OAttribute|GetHP))) true true "(R=1.000000,G=0.000000,B=0.000000,A=1.000000)" (Utilities|Time|GetWorldDeltaSeconds)))

(event EventBeginPlay
  (Default|Init (Variables|Default|GetBP_BuildingGridManagerComp)))

(event Input|AxisEvents|InputAxisMoveForward
  (params (AxisValue :type Float%20%28single-precision%29))
  ;[1 1 1] 位移逻辑
  (if (Variables|Status|GetCanMove)
    (CallFunction|MoveFunction AxisValue (stale Input|AxisEvents|InputAxisMoveRight AxisValue))))

(event Input|AxisEvents|InputAxisMoveRight
  (params (AxisValue :type Float%20%28single-precision%29))
  ;[1 1 1] 位移逻辑
  (if (Variables|Status|GetCanMove)
    (CallFunction|MoveFunction (stale Input|AxisEvents|InputAxisMoveForward AxisValue) AxisValue)))

(fn ConstructionScript
  (bind _floatingpawnmovement (Variables|Default|GetFloatingPawnMovement))
  (bind _floatingpawnmovement_2 (Variables|Default|GetFloatingPawnMovement))
  (Utilities|FlowControl|Sequence
    (:then_0
      (switch Utilities|FlowControl|Switch|SwitchonE_MovementMethod (Variables|OAttribute|GetMovementMethod)
        (:NewEnumerator0
          (Variables|/Script/Engine.FloatingPawnMovement|SetAcceleration _floatingpawnmovement_2 1.2e+03)
          (Variables|/Script/Engine.FloatingPawnMovement|SetDeceleration _floatingpawnmovement_2 8e+03)
          (Variables|/Script/Engine.FloatingPawnMovement|SetTurningBoost _floatingpawnmovement_2 8.0))
        (:NewEnumerator1
          (Variables|/Script/Engine.FloatingPawnMovement|SetAcceleration _floatingpawnmovement 3e+02 :!label _label)
          (Variables|/Script/Engine.FloatingPawnMovement|SetDeceleration _floatingpawnmovement 1e+03)
          (Variables|/Script/Engine.FloatingPawnMovement|SetTurningBoost _floatingpawnmovement 1.0))
        (:NewEnumerator2
          (goto _label))))))

(fn Loot
  (params (LootAmount :type Integer) (Loot :type Boolean%20%28by%20ref%29) (Coin :type Boolean%20%28by%20ref%29) (Exp :type Boolean%20%28by%20ref%29))
  (bind _asbp_gm_castle (Utilities|Casting|CastToBP_GM_Castle (Game|GetGameMode)))
  (Utilities|FlowControl|Sequence
    (:then_0
      (if Loot
        (Variables|/Game/BP/GM/BP_GM_Castle.BP_GM_Castle_C|SetCurrentMoney _asbp_gm_castle (+ (Variables|/Game/BP/GM/BP_GM_Castle.BP_GM_Castle_C|GetCurrentMoney _asbp_gm_castle) LootAmount))))
    (:then_1
      (if Coin
        _))
    (:then_2
      (if Exp
        _))
    (:then_3
      (CallFunction|LootEvent))))

(fn LootEvent)

(fn UpdateCollision
  (bind _collectarea (Variables|Default|GetCollectArea))
  (Components|Sphere|SetSphereRadius _collectarea (* (Variables|/Script/Engine.SphereComponent|GetSphereRadius _collectarea) (Math|Float|%(Float) (Variables|HAttribute|GetLootRadiusPct) 1.0)) true))

(fn DamagedEvent
  (params (Damage%20Type :type Damage%20Type%20Object%20Reference) (Damage%20Causer :type Actor%20Object%20Reference)))

(fn LevelUp)

(fn MoveFunction
  (params (ForwardValue :type Float%20%28double-precision%29) (RightValue :type Float%20%28double-precision%29))
  (LocalVariables|SetForwardValue_Local ForwardValue)
  (LocalVariables|SetRightValue_Local RightValue)
  (switch Utilities|FlowControl|Switch|SwitchonE_MovementMethod (Variables|OAttribute|GetMovementMethod)
    (:NewEnumerator0
      (|DirectlyMove))
    (:NewEnumerator1
      (|Tank))
    (:NewEnumerator2
      (|Drone))))