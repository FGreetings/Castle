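; Base castle construction that acts as an auto-firing tower against BP_EnemyBase actors within a configurable Range sphere.
; Overlaps maintain EnemiesInRange; Tick picks a random or nearest target, though the nearest search starts at zero distance so never updates its index.
; It yaws an Arrow toward the target, and a looping timer spawns bullets there, clearing the target after each shot.
; A dynamic-material marker shows build validity in green or red.
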(event OnComponentBeginOverlap(Sphere)
  (params (OverlappedComponent :type Primitive%20Component%20Object%20Reference) (OtherActor :type Actor%20Object%20Reference) (OtherComp :type Primitive%20Component%20Object%20Reference) (OtherBodyIndex :type Integer) (bFromSweep :type Boolean) (SweepResult :type Hit%20Result%20Structure%20%28by%20ref%29))
  ;[1 1 1] Add&RemoveEnemies
  (bind _asbp_enemy_base (Utilities|Casting|CastToBP_EnemyBase OtherActor))
  (Utilities|Array|Add (Variables|Default|GetEnemiesInRange) _asbp_enemy_base))

(event OnComponentEndOverlap(Sphere)
  (params (OverlappedComponent :type Primitive%20Component%20Object%20Reference) (OtherActor :type Actor%20Object%20Reference) (OtherComp :type Primitive%20Component%20Object%20Reference) (OtherBodyIndex :type Integer))
  ;[1 1 1] Add&RemoveEnemies
  (bind _asbp_enemy_base (Utilities|Casting|CastToBP_EnemyBase OtherActor))
  (Utilities|Array|RemoveItem (Variables|Default|GetEnemiesInRange) _asbp_enemy_base))

(event Custom|ShotEvent
  (Variables|Default|GetEnemyRef
    (:then
      (bind _returnvalue (Game|SpawnActorfromClass (Variables|Default|GetBulletClass) (Transformation|GetWorldTransform (Variables|Default|GetArrow)) "Undefined" 0 0 0))
      (Utilities|IsValid _returnvalue
        (:Is%20Valid
          (Variables|/Game/BP/Bullet/BP_BulletBase.BP_BulletBase_C|SetTarget _returnvalue (Variables|Default|GetEnemyRef))
          (Variables|Default|SetEnemyRef 0))))
    (:else)))

(event EventBeginPlay
  (Utilities|FlowControl|Sequence
    (:then_0
      (Utilities|Time|SetTimerbyFunctionName 0 "ShotEvent" (Variables|Default|GetShotingGap) true))
    (:then_1
      (Utilities|FlowControl|Delay 0.1)
      (Utilities|Array|AppendArray (Variables|Default|GetEnemiesInRange) (Collision|GetOverlappingActors (Variables|Default|GetSphere) "/Game/BP/Enemy/BP_EnemyBase.BP_EnemyBase_C" :!class /Script/Engine.PrimitiveComponent)))
    (:then_2
      (bind _returnvalue (Rendering|Material|CreateDynamicMaterialInstance (Variables|Default|GetConstructionStateMarker) 0 "/Game/Mat/M_BaseColor_ECRed.M_BaseColor_ECRed" "None" :!class /Script/Engine.PrimitiveComponent))
      (Variables|Default|SetMarkerMI _returnvalue))))

(event EventTick
  (params (DeltaSeconds :type Float%20%28single-precision%29))
  (Variables|Default|GetEnemyRef
    (:then
      _)
    (:else
      (CallFunction|FindEnemyAcordingtoType)))
  (CallFunction|AimtoEnemy))

(fn ConstructionScript
  (Components|Sphere|SetSphereRadius (Variables|Default|GetSphere) (Variables|Default|GetRange) true))

(fn FindEnemyAcordingtoType
  (switch Utilities|FlowControl|Switch|SwitchonE_AimingType (Variables|Default|GetAimingType)
    (:NewEnumerator0
      (CallFunction|FindEnemyRandomly))
    (:NewEnumerator1
      (CallFunction|FindNearestEnemy))))

(fn FindEnemyRandomly
  (Variables|Default|SetEnemyRef (Utilities|Array|Get(acopy) (Variables|Default|GetEnemiesInRange) (Math|Random|RandomInteger (Utilities|Array|Length (Variables|Default|GetEnemiesInRange))))))

(fn FindNearestEnemy
  (bind _enemiesinrange (Variables|Default|GetEnemiesInRange))
  (LocalVariables|SetNearestDistance 0.0)
  (for (_array_element _array_index) _enemiesinrange
    (if (< (Math|Vector|Distance2D(Vector) (Transformation|GetActorLocation _array_element) (Transformation|GetActorLocation)) (LocalVariables|GetNearestDistance))
      (LocalVariables|SetNearestDistance (Math|Vector|Distance2D(Vector) (Transformation|GetActorLocation _array_element) (Transformation|GetActorLocation)))
      (LocalVariables|SetIndex _array_index)))
  (Variables|Default|SetEnemyRef (Utilities|Array|Get(acopy) _enemiesinrange (LocalVariables|GetIndex))))

(fn AimtoEnemy
  (bind _arrow (Variables|Default|GetArrow))
  (bind _enemyref (Variables|Default|GetEnemyRef))
  (Utilities|IsValid _enemyref
    (:Is%20Valid
      (Transformation|SetWorldRotation _arrow (Math|Rotator|MakeRotator 0.0 0.0 (.Yaw (Math|Rotator|BreakRotator (Math|Rotator|FindLookatRotation (Transformation|GetWorldLocation _arrow) (Transformation|GetActorLocation _enemyref))))) false false))))

(fn UpdateBuildingStateMarker
  (params (InBuildState :type Boolean) (CanBuild :type Boolean))
  (Rendering|SetVisibility (Variables|Default|GetConstructionStateMarker) InBuildState false)
  (Rendering|Material|SetVectorParameterValue (Variables|Default|GetMarkerMI) "EC" (select CanBuild "(R=0.000000,G=20.000000,B=0.000000,A=1.000000)" "(R=20.000000,G=0.000000,B=0.000000,A=1.000000)") :!class /Script/Engine.MaterialInstanceDynamic))