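; Castle building-grid component that spawns a hexagonal field of BP_BuildingGridBase cells around its owner, attached to the BP_CastleBase's Base.
; PopulateGrid builds concentric rings up to Round, placing cells on six computed corners and interpolating along edges, while stepping axial hex indices stored in HexGridArray.
; GetClosestGridLocation linearly searches that array for the nearest cell by 2D distance.
; An older rectangular-grid layout remains as disconnected, never-run logic.
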(event Custom|Init)

(fn PopulateGrid
  (bind _returnvalue (Components|GetOwner))
  (bind _returnvalue_2 (Transformation|GetActorLocation _returnvalue))
  (bind (_x _y _z) (Math|Vector|BreakVector _returnvalue_2))
  (LocalVariables|SetGridLongDiameter (* (Variables|Default|GetGridShortDiameter) (Math|Trig|Cos(Degrees) 3e+01)))
  (Utilities|Array|Clear (Variables|Default|GetHexGridArray))
  (for _index (range 0 (Variables|Default|GetRound))
    (bind _output_get (LocalVariables|SetCurrentRoundIndex _index))
    (if (== _output_get 0)
      ;[1 1 1] 生成中心格
      (bind _returnvalue_3 (Game|SpawnActorfromClass "/Game/BP/Castle/BP_BuildingGridBase.BP_BuildingGridBase_C" (Math|Transform|MakeTransform (Math|Vector|MakeVector _x _y _z) "0, 0, 0" "1.000000,1.000000,1.000000") "Undefined" 0 false (Utilities|Struct|MakeStruct_HexIndex) 0))
      (bind _asbp_castle_base (Utilities|Casting|CastToBP_CastleBase (Components|GetOwner)))
      (Transformation|AttachComponentToComponent _returnvalue_3 (Variables|/Game/BP/Castle/BP_CastleBase.BP_CastleBase_C|GetBase _asbp_castle_base) "None" "KeepWorld" "KeepRelative" "KeepWorld" true)
      (Utilities|Array|AddUnique (Variables|Default|GetHexGridArray) (Utilities|Struct|MakeStruct_HexReference _returnvalue_3 (Utilities|Struct|MakeStruct_HexIndex)))
      (else
        ;[1 1 1] 计算顶点
        (LocalVariables|SetCurrentRoundRadius (* (Variables|Default|GetGridShortDiameter) (LocalVariables|GetCurrentRoundIndex)))
        (Utilities|Array|Clear (LocalVariables|GetHexApex))
        (for _index_2 (range 0 5)
          (Utilities|Array|Add (LocalVariables|GetHexApex) (Math|Vector|MakeVector (* (Math|Trig|Cos(Degrees) (Math|Conversions|ToFloat(Integer) (- (* _index_2 60) 120))) (LocalVariables|GetCurrentRoundRadius)) (* (Math|Trig|Sin(Degrees) (Math|Conversions|ToFloat(Integer) (- (* _index_2 60) 120))) (LocalVariables|GetCurrentRoundRadius)) 0.0)))
        ;[1 1 1] 计算Index
        (for _index_3 (range 0 (- (* (LocalVariables|GetCurrentRoundIndex) 6) 1))
          (bind _output_get_2 (LocalVariables|SetCurrentGridIndex _index_3))
          (if (== _output_get_2 0)
            (LocalVariables|SetCurrentHexIndex (Utilities|Struct|MakeStruct_HexIndex 0 (- 0 (LocalVariables|GetCurrentRoundIndex))))
            (else
              (switch int (Math|Float|Ceil (/ (LocalVariables|GetCurrentGridIndex) (LocalVariables|GetCurrentRoundIndex)))
                (:1
                  (LocalVariables|SetCurrentHexIndex (Utilities|Struct|MakeStruct_HexIndex (+ (.X (Utilities|Struct|BreakStruct_HexIndex (LocalVariables|GetCurrentHexIndex))) 1) (.Y (Utilities|Struct|BreakStruct_HexIndex (LocalVariables|GetCurrentHexIndex))))))
                (:2
                  (LocalVariables|SetCurrentHexIndex (Utilities|Struct|MakeStruct_HexIndex (.X (Utilities|Struct|BreakStruct_HexIndex (LocalVariables|GetCurrentHexIndex))) (+ (.Y (Utilities|Struct|BreakStruct_HexIndex (LocalVariables|GetCurrentHexIndex))) 1))))
                (:3
                  (LocalVariables|SetCurrentHexIndex (Utilities|Struct|MakeStruct_HexIndex (- (.X (Utilities|Struct|BreakStruct_HexIndex (LocalVariables|GetCurrentHexIndex))) 1) (+ (.Y (Utilities|Struct|BreakStruct_HexIndex (LocalVariables|GetCurrentHexIndex))) 1))))
                (:4
                  (LocalVariables|SetCurrentHexIndex (Utilities|Struct|MakeStruct_HexIndex (- (.X (Utilities|Struct|BreakStruct_HexIndex (LocalVariables|GetCurrentHexIndex))) 1) (.Y (Utilities|Struct|BreakStruct_HexIndex (LocalVariables|GetCurrentHexIndex))))))
                (:5
                  (LocalVariables|SetCurrentHexIndex (Utilities|Struct|MakeStruct_HexIndex (.X (Utilities|Struct|BreakStruct_HexIndex (LocalVariables|GetCurrentHexIndex))) (- (.Y (Utilities|Struct|BreakStruct_HexIndex (LocalVariables|GetCurrentHexIndex))) 1))))
                (:6
                  (LocalVariables|SetCurrentHexIndex (Utilities|Struct|MakeStruct_HexIndex (+ (.X (Utilities|Struct|BreakStruct_HexIndex (LocalVariables|GetCurrentHexIndex))) 1) (- (.Y (Utilities|Struct|BreakStruct_HexIndex (LocalVariables|GetCurrentHexIndex))) 1)))))))
          (if (== (Math|Integer|%(Integer) (LocalVariables|GetCurrentGridIndex) (LocalVariables|GetCurrentRoundIndex)) 0)
            ;[1 1 1] 计算位置并生成（顶点）
            (bind _returnvalue_4 (Game|SpawnActorfromClass "/Game/BP/Castle/BP_BuildingGridBase.BP_BuildingGridBase_C" (Math|Transform|MakeTransform (Math|Vector|MakeVector (.X (Math|Vector|BreakVector (+ (Utilities|Array|Get(acopy) (LocalVariables|GetHexApex) (/ (LocalVariables|GetCurrentGridIndex) (LocalVariables|GetCurrentRoundIndex))) (Transformation|GetActorLocation (Components|GetOwner))))) (.Y (Math|Vector|BreakVector (+ (Utilities|Array|Get(acopy) (LocalVariables|GetHexApex) (/ (LocalVariables|GetCurrentGridIndex) (LocalVariables|GetCurrentRoundIndex))) (Transformation|GetActorLocation (Components|GetOwner))))) (.Z (Math|Vector|BreakVector (+ (Utilities|Array|Get(acopy) (LocalVariables|GetHexApex) (/ (LocalVariables|GetCurrentGridIndex) (LocalVariables|GetCurrentRoundIndex))) (Transformation|GetActorLocation (Components|GetOwner)))))) "0, 0, 0" "1.000000,1.000000,1.000000") "Undefined" 0 false (LocalVariables|GetCurrentHexIndex) 0))
            (bind _asbp_castle_base_2 (Utilities|Casting|CastToBP_CastleBase (Components|GetOwner)))
            (Transformation|AttachComponentToComponent _returnvalue_4 (Variables|/Game/BP/Castle/BP_CastleBase.BP_CastleBase_C|GetBase _asbp_castle_base_2) "None" "KeepWorld" "KeepRelative" "KeepWorld" true)
            (Utilities|Array|AddUnique (Variables|Default|GetHexGridArray) (Utilities|Struct|MakeStruct_HexReference _returnvalue_4 (LocalVariables|GetCurrentHexIndex)))
            (else
              ;[1 1 1] 计算位置并生成（非顶点）
              (bind _next (CallFunction|GetNextNum (Math|Float|Floor (/ (LocalVariables|GetCurrentGridIndex) (LocalVariables|GetCurrentRoundIndex)))))
              (bind _returnvalue_5 (Game|SpawnActorfromClass "/Game/BP/Castle/BP_BuildingGridBase.BP_BuildingGridBase_C" (Math|Transform|MakeTransform (Math|Vector|MakeVector (.X (Math|Vector|BreakVector (+ (+ (Utilities|Array|Get(acopy) (LocalVariables|GetHexApex) (Math|Float|Floor (/ (LocalVariables|GetCurrentGridIndex) (LocalVariables|GetCurrentRoundIndex)))) (* (Math|Vector|Normalize (- (Utilities|Array|Get(acopy) (LocalVariables|GetHexApex) _next) (Utilities|Array|Get(acopy) (LocalVariables|GetHexApex) (Math|Float|Floor (/ (LocalVariables|GetCurrentGridIndex) (LocalVariables|GetCurrentRoundIndex)))))) (* (LocalVariables|GetCurrentRoundRadius) (/ (Math|Integer|%(Integer) (LocalVariables|GetCurrentGridIndex) (LocalVariables|GetCurrentRoundIndex)) (Math|Conversions|ToFloat(Integer) (LocalVariables|GetCurrentRoundIndex)))))) (Transformation|GetActorLocation (Components|GetOwner))))) (.Y (Math|Vector|BreakVector (+ (+ (Utilities|Array|Get(acopy) (LocalVariables|GetHexApex) (Math|Float|Floor (/ (LocalVariables|GetCurrentGridIndex) (LocalVariables|GetCurrentRoundIndex)))) (* (Math|Vector|Normalize (- (Utilities|Array|Get(acopy) (LocalVariables|GetHexApex) _next) (Utilities|Array|Get(acopy) (LocalVariables|GetHexApex) (Math|Float|Floor (/ (LocalVariables|GetCurrentGridIndex) (LocalVariables|GetCurrentRoundIndex)))))) (* (LocalVariables|GetCurrentRoundRadius) (/ (Math|Integer|%(Integer) (LocalVariables|GetCurrentGridIndex) (LocalVariables|GetCurrentRoundIndex)) (Math|Conversions|ToFloat(Integer) (LocalVariables|GetCurrentRoundIndex)))))) (Transformation|GetActorLocation (Components|GetOwner))))) (.Z (Math|Vector|BreakVector (+ (+ (Utilities|Array|Get(acopy) (LocalVariables|GetHexApex) (Math|Float|Floor (/ (LocalVariables|GetCurrentGridIndex) (LocalVariables|GetCurrentRoundIndex)))) (* (Math|Vector|Normalize (- (Utilities|Array|Get(acopy) (LocalVariables|GetHexApex) _next) (Utilities|Array|Get(acopy) (LocalVariables|GetHexApex) (Math|Float|Floor (/ (LocalVariables|GetCurrentGridIndex) (LocalVariables|GetCurrentRoundIndex)))))) (* (LocalVariables|GetCurrentRoundRadius) (/ (Math|Integer|%(Integer) (LocalVariables|GetCurrentGridIndex) (LocalVariables|GetCurrentRoundIndex)) (Math|Conversions|ToFloat(Integer) (LocalVariables|GetCurrentRoundIndex)))))) (Transformation|GetActorLocation (Components|GetOwner)))))) "0, 0, 0" "1.000000,1.000000,1.000000") "Undefined" 0 false (LocalVariables|GetCurrentHexIndex) 0))
              (bind _asbp_castle_base_3 (Utilities|Casting|CastToBP_CastleBase (Components|GetOwner)))
              (Transformation|AttachComponentToComponent _returnvalue_5 (Variables|/Game/BP/Castle/BP_CastleBase.BP_CastleBase_C|GetBase _asbp_castle_base_3) "None" "KeepWorld" "KeepRelative" "KeepWorld" true)
              (Utilities|Array|AddUnique (Variables|Default|GetHexGridArray) (Utilities|Struct|MakeStruct_HexReference _returnvalue_5 (LocalVariables|GetCurrentHexIndex))))))))))

(fn GetClosestGridLocation
  (params (InPosition :type Vector))
  (for _array_element (Variables|Default|GetHexGridArray)
    (if (< (Math|Vector|Distance2D(Vector) (Transformation|GetActorLocation (.HexGrid (Utilities|Struct|BreakStruct_HexReference _array_element))) InPosition) (LocalVariables|GetClosestDistance_Local))
      (LocalVariables|SetClosestDistance_Local (Math|Vector|Distance2D(Vector) (Transformation|GetActorLocation (.HexGrid (Utilities|Struct|BreakStruct_HexReference _array_element))) InPosition))
      (LocalVariables|SetClosestLocation_Local (Transformation|GetActorLocation (.HexGrid (Utilities|Struct|BreakStruct_HexReference _array_element))))
      (LocalVariables|SetClosestGrid_local (.HexGrid (Utilities|Struct|BreakStruct_HexReference _array_element)))))
  (return (LocalVariables|GetClosestGrid_local) (LocalVariables|GetClosestLocation_Local) (LocalVariables|GetClosestDistance_Local)))

(fn AttributeIndex)

(fn GetNextNum
  (params (Current :type Integer))
  (if (>= Current 5)
    (return 0)
    (else
      (return (+ Current 1)))))